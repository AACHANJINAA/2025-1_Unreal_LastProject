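; BP_ThrowKnife_PickUp is a pickup actor that grants the throwing knife skill to the BP_Assasin player character.
; A widget component shows a beckoning prompt from BeginPlay, switching to a key prompt while the assassin overlaps the sphere.
; The Interactor event casts the caller to BP_Assasin, calls AcquireThrowingKnifeSkill and destroys the pickup.
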(event `self.ReceiveBeginPlay`
  (bind _aswbp_throw_knife_pick_up (cast `/Game/Main/Throw/WBP_ThrowKnife_PickUp` (`WidgetComponent.GetUserWidgetObject` (`self.WBP`))))
  (`/Game/Main/Throw/WBP_ThrowKnife_PickUp.UpdateText` _aswbp_throw_knife_pick_up "COME HERE!!")
  (`SceneComponent.SetVisibility` (`self.WBP`) true false))

(event `/Game/Main/BPI_Interact.Interactor`
  (params (Interactor :type "Actor Object Reference"))
  (bind _asbp_assasin (cast `/Game/Main/BP_Assasin` Interactor))
  (`/Game/Main/BP_Assasin.AcquireThrowingKnifeSkill` _asbp_assasin)
  (`self.K2_DestroyActor`))

(event `self.Sphere.OnComponentBeginOverlap`
  (params (OverlappedComponent :type "PrimitiveComponent Object Reference") (OtherActor :type "Actor Object Reference") (OtherComp :type "PrimitiveComponent Object Reference") (OtherBodyIndex :type Integer) (bFromSweep :type Boolean) (SweepResult :type "HitResult Structure (by ref)"))
  (cast `/Game/Main/BP_Assasin` OtherActor)
  (bind _aswbp_throw_knife_pick_up (cast `/Game/Main/Throw/WBP_ThrowKnife_PickUp` (`WidgetComponent.GetUserWidgetObject` (`self.WBP`))))
  (`/Game/Main/Throw/WBP_ThrowKnife_PickUp.UpdateText` _aswbp_throw_knife_pick_up "Press 'E'"))

(event `self.Sphere.OnComponentEndOverlap`
  (params (OverlappedComponent :type "PrimitiveComponent Object Reference") (OtherActor :type "Actor Object Reference") (OtherComp :type "PrimitiveComponent Object Reference") (OtherBodyIndex :type Integer))
  (cast `/Game/Main/BP_Assasin` OtherActor)
  (`/Game/Main/Throw/WBP_ThrowKnife_PickUp.UpdateText` (stale `self.Sphere.OnComponentBeginOverlap` _aswbp_throw_knife_pick_up) "COME HERE!!"))

(fn `UserConstructionScript`)