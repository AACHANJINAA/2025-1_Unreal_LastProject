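; Assassin character Blueprint with input-driven movement, jumping, interface-based interaction, a throwing knife and a sword attack.
; The knife unlocks through AcquireThrowingKnifeSkill; Q plays the throw montage with a short cooldown, and a separate event spawns the projectile ahead of the hand socket.
; R plays the sword montage, while separate events toggle sword collision, whose DoOnce-gated overlap sends damage through a message call.
; Tick stores horizontal speed.
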(event `self.ReceiveBeginPlay`
  (set `self.bCanThrowKnife` false)
  (`ActorComponent.Deactivate` (`self.Sword_Collision`))
  (set `self.bCanUseSword` true)
  (set `self.bIsAttacking` false))

(event `self.ReceiveTick`
  (params (DeltaSeconds :type "Float (single-precision)"))
  (set `self.Speed` (`KismetMathLibrary.VSizeXY` (`self.GetVelocity`))))

(event `EnhancedInput|/Game/ThirdPerson/Input/Actions/IA_Move`
  (params (ActionValue :type "Vector2D Structure") (ElapsedSeconds :type "Float (double-precision)") (TriggeredSeconds :type "Float (double-precision)") (InputAction :type "InputAction Object Reference" :default "/Game/ThirdPerson/Input/Actions/IA_Move.IA_Move"))
  (bind (_returnvalue_roll _returnvalue_pitch _returnvalue_yaw) (`KismetMathLibrary.BreakRotator` (`self.GetControlRotation`)))
  (bind _returnvalue (`KismetMathLibrary.MakeRotator` 0.0 0.0 _returnvalue_yaw))
  (:`Triggered`
    (`self.AddMovementInput` (`KismetMathLibrary.GetRightVector` _returnvalue) ActionValue_X)
    (`self.AddMovementInput` (`KismetMathLibrary.GetForwardVector` _returnvalue) ActionValue_Y)))

(event `EnhancedInput|/Game/ThirdPerson/Input/Actions/IA_Jump`
  (params (ActionValue :type Boolean) (ElapsedSeconds :type "Float (double-precision)") (TriggeredSeconds :type "Float (double-precision)") (InputAction :type "InputAction Object Reference" :default "/Game/ThirdPerson/Input/Actions/IA_Jump.IA_Jump"))
  (:`Started`
    (`self.Jump`)))

(event `Key|Q`
  (params (Key :type "Key Structure"))
  (:`Pressed`
    (if (and (`self.bCanThrowKnife`) (not (`self.bIsAttacking`)))
      (`SceneComponent.SetVisibility` (`self.HandDagger_Visual`) false false)
      (`self.PlayAnimMontage` "/Game/Main/Weapon/AM_ThrowKnife.AM_ThrowKnife")
      (set `self.bCanThrowKnife` false)
      (`KismetSystemLibrary.Delay` 0.5)
      (set `self.bCanThrowKnife` true)
      (`SceneComponent.SetVisibility` (`self.Mesh`) true false))))

(event `ExcuteKnifeSpawn`
  (bind _returnvalue (`self.K2_GetActorRotation`))
  (`|SpawnActorFromClass` "/Game/Main/Weapon/BP_Throw_Knife.BP_Throw_Knife_C" (`KismetMathLibrary.MakeTransform` (+ (`SceneComponent.GetSocketLocation` (`self.HandDagger_Visual`) "Throw_Knife") (* (`KismetMathLibrary.GetForwardVector` _returnvalue) 200.0)) _returnvalue) "AlwaysSpawn" "MultiplyWithRoot" null null))

(event `Key|E`
  (params (Key :type "Key Structure"))
  (:`Pressed`
    (for _array_element (`self.GetOverlappingActors` null)
      (if (`KismetSystemLibrary.DoesImplementInterface` _array_element "/Game/Main/BPI_Interact.BPI_Interact_C")
        (message `/Game/Main/BPI_Interact.Interactor` _array_element self)))))

(event `AcquireThrowingKnifeSkill`
  (set `self.bCanThrowKnife` true)
  (`SceneComponent.SetVisibility` (`self.HandDagger_Visual`) true false))

(event `Key|R`
  (params (Key :type "Key Structure"))
  (:`Pressed`
    (if (and (`self.bCanUseSword`) (not (`self.bIsAttacking`)))
      (`self.PlayAnimMontage` "/Game/Main/Weapon/AM_Sword.AM_Sword"))))

(event `ActivateSwordCollision`
  (`ActorComponent.Activate` (`self.Sword_Collision`) false :!label _label)
  (`/Engine/EditorBlueprintResources/StandardMacros.DoOnce` false
    (:`Completed`
      (goto _label))))

(event `DisableSwordCollision`
  (`ActorComponent.Deactivate` (`self.Sword_Collision`))
  (set `self.bIsAttacking` false))

(event `self.Sword_Collision.OnComponentBeginOverlap`
  (params (OverlappedComponent :type "PrimitiveComponent Object Reference") (OtherActor :type "Actor Object Reference") (OtherComp :type "PrimitiveComponent Object Reference") (OtherBodyIndex :type Integer) (bFromSweep :type Boolean) (SweepResult :type "HitResult Structure (by ref)"))
  (`/Engine/EditorBlueprintResources/StandardMacros.DoOnce` false
    (:`Completed`
      (if (!= OtherActor (`self.GetInstigator`))
        (message `/Game/Main/BPI_Damagable.ApplyDamage` OtherActor (`self.GetInstigator`) 10.0)))))

(fn `UserConstructionScript`)