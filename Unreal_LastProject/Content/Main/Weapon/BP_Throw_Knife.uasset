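; BP_Throw_Knife is a thrown knife weapon actor that damages what it hits.
; On BeginPlay it adds 90 degrees of pitch to its rotation.
; When its Capsule begins overlapping anything other than a BP_Assasin, it prints that actor's name, plays a sound, applies a small fixed damage and destroys itself.
; The graph contains no movement logic.
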(event `self.ReceiveBeginPlay`
  (bind (_returnvalue_roll _returnvalue_pitch _returnvalue_yaw) (`KismetMathLibrary.BreakRotator` (`self.K2_GetActorRotation`)))
  (`self.K2_SetActorRotation` (`KismetMathLibrary.MakeRotator` _returnvalue_roll (+ _returnvalue_pitch 90.0) _returnvalue_yaw)))

(event `self.Capsule.OnComponentBeginOverlap`
  (params (OverlappedComponent :type "PrimitiveComponent Object Reference") (OtherActor :type "Actor Object Reference") (OtherComp :type "PrimitiveComponent Object Reference") (OtherBodyIndex :type Integer) (bFromSweep :type Boolean) (SweepResult :type "HitResult Structure (by ref)"))
  (cast `/Game/Main/Assasin_BP/BP_Assasin` OtherActor
    (:`CastFailed`
      (`KismetSystemLibrary.PrintString` (`KismetSystemLibrary.GetDisplayName` OtherActor))
      (`GameplayStatics.PlaySoundAtLocation` "/Game/ShortSound/cue/Bag_Handle_1-5_Cue.Bag_Handle_1-5_Cue" (`self.K2_GetActorLocation`) (struct) 1.0 1.0 0.0 null null null null)
      (`GameplayStatics.ApplyDamage` OtherActor 0.5 null self)
      (`self.K2_DestroyActor`))))

(fn `UserConstructionScript`)