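; BP_Mutant is a mutant monster pawn that wanders the navmesh at random.
; From BeginPlay it loops AI MoveTo calls to random navigable points around its current location, playing a success or failure sound and printing the result before repeating.
; ApplyDamage is an empty event; the logic that would decrease BPHealthComponent health and set IsDead on ABP_Mutant is disconnected and never runs.
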(event `self.ReceiveBeginPlay`
  (bind (_randomlocation _returnvalue) (`NavigationSystemV1.K2_GetRandomLocationInNavigableRadius` (`self.K2_GetActorLocation`) 1000.0 null null :!label _label))
  (if _returnvalue
    (bind _movementresult (`|AIMoveTo` self _randomlocation null 50.0)
      (:`OnSuccess`
        (`GameplayStatics.PlaySound2D` "/Engine/VREditor/Sounds/UI/Click_on_Button.Click_on_Button" 1.0 1.0 0.0 null null))
      (:`OnFail`
        (`GameplayStatics.PlaySound2D` "/Engine/EditorSounds/Notifications/CompileFailed.CompileFailed" 1.0 1.0 0.0 null null)))
    (`KismetSystemLibrary.PrintString` (`|GetEnumeratorNameAsString` _movementresult))
    (goto _label)))

(event `/Game/Main/BPI_Damagable.ApplyDamage`
  (params (DamageCauser :type "Actor Object Reference") (Damage :type "Float (double-precision)")))

(fn `UserConstructionScript`)