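; Basic mutant enemy that hurts the BP_Assasin player on contact and can be killed by damage.
; Sphere overlap with the assassin either relocates the mutant, depending on a KickCollision check, or applies damage to the player.
; Incoming damage lowers HP and shifts a dynamic material tint from black to red.
; At zero HP it reports a kill to BP_AssasinGameMode, plays a death montage, then destroys itself with sound and steam effects.
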(event `self.ReceiveBeginPlay`
  (bind _returnvalue (`PrimitiveComponent.CreateDynamicMaterialInstance` (`self.Mesh`) 0 null "None"))
  (set `self.DynamicMaterial` _returnvalue))

(event `self.ReceiveAnyDamage`
  (params (Damage :type "Float (single-precision)") (DamageType :type "DamageType Object Reference") (InstigatedBy :type "Controller Object Reference") (DamageCauser :type "Actor Object Reference"))
  (bind _returnvalue (`self.K2_GetActorLocation`))
  (bind _output_get (set `self.HP` (- (`self.HP`) Damage)))
  (`MaterialInstanceDynamic.SetVectorParameterValue` (`self.DynamicMaterial`) "BodyTintColor" (`KismetMathLibrary.LinearColorLerp` (struct :`A` 1.0) (struct :`R` 1.0 :`A` 1.0) (- 1.0 (/ (`self.HP`) 1.0))))
  (if (<= _output_get 0.0)
    (bind _asbp_assasin_game_mode (cast `/Game/Main/Assasin_BP/BP_AssasinGameMode` (`GameplayStatics.GetGameMode`)))
    (`/Game/Main/Assasin_BP/BP_AssasinGameMode.AddKillCount` _asbp_assasin_game_mode)
    (`self.PlayAnimMontage` "/Game/Main/Monster/MutantAnimation/AM_MutatntDIE.AM_MutatntDIE")
    (`KismetSystemLibrary.Delay` 1.0)
    (`self.K2_DestroyActor`)
    (`GameplayStatics.PlaySoundAtLocation` "/Game/ShortSound/wav/Hit_Generic_2-1.Hit_Generic_2-1" _returnvalue (struct) 1.0 1.0 0.0 null null null null)
    (`GameplayStatics.SpawnEmitterAtLocation` "/Game/StarterContent/Particles/P_Steam_Lit.P_Steam_Lit" _returnvalue)))

(event `self.Sphere.OnComponentBeginOverlap`
  (params (OverlappedComponent :type "PrimitiveComponent Object Reference") (OtherActor :type "Actor Object Reference") (OtherComp :type "PrimitiveComponent Object Reference") (OtherBodyIndex :type Integer) (bFromSweep :type Boolean) (SweepResult :type "HitResult Structure (by ref)"))
  (bind _asbp_assasin (cast `/Game/Main/Assasin_BP/BP_Assasin` OtherActor))
  (if (== (`/Game/Main/Assasin_BP/BP_Assasin.KickCollision` _asbp_assasin) null)
    (`self.K2_SetActorLocation` (`KismetMathLibrary.Normal` (- (`self.K2_GetActorLocation`) (`self.K2_GetActorLocation`)) 1.0))
    (else
      (`GameplayStatics.ApplyDamage` _asbp_assasin 0.1 null self))))

(fn `UserConstructionScript`)