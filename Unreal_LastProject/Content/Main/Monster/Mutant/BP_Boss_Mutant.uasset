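; Mutant boss enemy that attacks on proximity, damages the Assasin character on mesh overlap, and dies in an explosion.
; Damage lowers HP and drives the body tint through a dynamic material, using an alpha of MaxHP minus the HP ratio.
; AttackCollision overlaps trigger the attack montage while alive, and MeshCollision applies the damage.
; At zero HP it plays a death montage and sound, then destroys itself after a delay with explosion effects.
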(event `self.ReceiveBeginPlay`
  (bind _returnvalue (`PrimitiveComponent.CreateDynamicMaterialInstance` (`self.Mesh`) 0 null "None"))
  (set `self.DynamicMaterial` _returnvalue))

(event `self.ReceiveAnyDamage`
  (params (Damage :type "Float (single-precision)") (DamageType :type "DamageType Object Reference") (InstigatedBy :type "Controller Object Reference") (DamageCauser :type "Actor Object Reference"))
  (bind _returnvalue (`self.K2_GetActorLocation`))
  (bind _output_get (set `self.HP` (- (`self.HP`) Damage)))
  (`MaterialInstanceDynamic.SetVectorParameterValue` (`self.DynamicMaterial`) "BodyTintColor" (`KismetMathLibrary.LinearColorLerp` (struct :`A` 1.0) (struct :`R` 1.0 :`A` 1.0) (- (`self.Max_HP`) (/ (`self.HP`) (`self.Max_HP`)))))
  (if (<= _output_get 0.0)
    (`self.PlayAnimMontage` "/Game/Main/Assasin_BP/AM_AssasinDie.AM_AssasinDie")
    (`GameplayStatics.PlaySoundAtLocation` "/Game/StarterContent/Audio/Collapse01.Collapse01" _returnvalue (struct) 1.0 1.0 0.0 null null null null)
    (`KismetSystemLibrary.Delay` 2.0)
    (`self.K2_DestroyActor`)
    (`GameplayStatics.PlaySoundAtLocation` "/Game/StarterContent/Audio/Explosion01.Explosion01" _returnvalue (struct) 1.0 1.0 0.0 null null null null)
    (`GameplayStatics.SpawnEmitterAtLocation` "/Game/StarterContent/Particles/P_Explosion.P_Explosion" _returnvalue (struct) (3.0 3.0 3.0))))

(event `self.AttackCollision.OnComponentBeginOverlap`
  (params (OverlappedComponent :type "PrimitiveComponent Object Reference") (OtherActor :type "Actor Object Reference") (OtherComp :type "PrimitiveComponent Object Reference") (OtherBodyIndex :type Integer) (bFromSweep :type Boolean) (SweepResult :type "HitResult Structure (by ref)"))
  (if (not (<= (`self.HP`) 0.0))
    (`self.PlayAnimMontage` "/Game/Main/Monster/MutantAnimation/AM_BossMutantAttack.AM_BossMutantAttack")))

(event `self.MeshCollision.OnComponentBeginOverlap`
  (params (OverlappedComponent :type "PrimitiveComponent Object Reference") (OtherActor :type "Actor Object Reference") (OtherComp :type "PrimitiveComponent Object Reference") (OtherBodyIndex :type Integer) (bFromSweep :type Boolean) (SweepResult :type "HitResult Structure (by ref)"))
  (bind _asbp_assasin (cast `/Game/Main/Assasin_BP/BP_Assasin` OtherActor))
  (`GameplayStatics.ApplyDamage` _asbp_assasin 0.2 null self))

(fn `UserConstructionScript`)