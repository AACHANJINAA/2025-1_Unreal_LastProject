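; BP_AssasinGameMode is the game mode that tracks mutant kills and triggers the boss spawn.
; AddKillCount increments the kill counter and broadcasts the new total through the OnKillCountChanged dispatcher.
; Once the count reaches twelve, it spawns BP_Boss_Mutant a single time, guarded by both a DoOnce and an IsSpawn flag.
; The event graph and construction script contain no logic.
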(fn `AddKillCount`
  (bind _result (`/Engine/EditorBlueprintResources/StandardMacros.IncrementInt` (`self.MutantKillCount`))
    (:`  `
      (bind _output_get (set `self.MutantKillCount` _result))
      (`self.OnKillCountChanged` (`self.MutantKillCount`))
      (if (>= _output_get 12)
        (if (not (`self.bIsSpawn`))
          (`/Engine/EditorBlueprintResources/StandardMacros.DoOnce` false
            (:`Completed`
              (`|SpawnActorFromClass` "/Game/Main/Monster/Mutant/BP_Boss_Mutant.BP_Boss_Mutant_C" (`self.Spawn Transform`) "Undefined" "MultiplyWithRoot" null null)
              (set `self.bIsSpawn` true))))))))

(fn `UserConstructionScript`)