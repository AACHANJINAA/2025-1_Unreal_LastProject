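; Player assassin character with movement, jump, a right-mouse over-the-shoulder aim mode and interface-based interaction with overlapping actors.
; OnSword, OnDagger and OffWeapon switch loadouts by toggling ability flags, visibility, sword collision and walk speed, via keys or skill-acquisition events that also restyle UI_Assasin buttons.
; Attacks play montages, with separate events spawning knives and toggling sword collision, which damages overlapped actors.
; Incoming damage reduces HP, triggering hit reactions or death and destruction.
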(event `self.ReceiveBeginPlay`
  (bind _returnvalue (`GameplayStatics.GetPlayerController` 0))
  (set `PlayerController.bShowMouseCursor` false _returnvalue)
  (`WidgetBlueprintLibrary.SetInputMode_GameOnly` _returnvalue true)
  (bind _output_get (set `self.Target HUD` (`PlayerController.GetHUD` _returnvalue)))
  (set `HUD.bShowHUD` false _output_get)
  (bind _returnvalue_2 (`|CreateWidget` "/Game/Main/Assasin_BP/UI_Assasin.UI_Assasin_C" null self))
  (`UserWidget.AddToViewport` _returnvalue_2 0)
  (`self.OffWeapon`)
  (set `self.bIsAttacking` false)
  (set `self.UI` _returnvalue_2))

(event `self.ReceiveTick`
  (params (DeltaSeconds :type "Float (single-precision)"))
  (set `self.Speed` (`KismetMathLibrary.VSizeXY` (`self.GetVelocity`))))

(event `EnhancedInput|/Game/ThirdPerson/Input/Actions/IA_Move`
  (params (ActionValue :type "Vector2D Structure") (ElapsedSeconds :type "Float (double-precision)") (TriggeredSeconds :type "Float (double-precision)") (InputAction :type "InputAction Object Reference" :default "/Game/ThirdPerson/Input/Actions/IA_Move.IA_Move"))
  (bind (_returnvalue_roll _returnvalue_pitch _returnvalue_yaw) (`KismetMathLibrary.BreakRotator` (`self.GetControlRotation`)))
  (bind _returnvalue (`KismetMathLibrary.MakeRotator` 0.0 0.0 _returnvalue_yaw))
  (:`Triggered`
    (`self.AddMovementInput` (`KismetMathLibrary.GetRightVector` _returnvalue) ActionValue_X)
    (`self.AddMovementInput` (`KismetMathLibrary.GetForwardVector` _returnvalue) ActionValue_Y)))

(event `EnhancedInput|/Game/ThirdPerson/Input/Actions/IA_Jump`
  (params (ActionValue :type Boolean) (ElapsedSeconds :type "Float (double-precision)") (TriggeredSeconds :type "Float (double-precision)") (InputAction :type "InputAction Object Reference" :default "/Game/ThirdPerson/Input/Actions/IA_Jump.IA_Jump"))
  (:`Started`
    (`self.Jump`)))

(event `Key|RightMouseButton`
  (params (Key :type "Key Structure"))
  (:`Pressed`
    (`self.Set Aim Mode`))
  (:`Released`
    (`self.Set Nav Mode`)))

(event `Key|Q`
  (params (Key :type "Key Structure"))
  (:`Pressed`
    (if (and (`self.bCanThrowKnife`) (not (`self.bIsAttacking`)))
      (`SceneComponent.SetVisibility` (`self.HandDagger_Visual`) false false)
      (`self.PlayAnimMontage` "/Game/Main/Weapon/AM_ThrowKnife.AM_ThrowKnife")
      (`GameplayStatics.PlaySoundAtLocation` "/Game/ShortSound/cue/Whoosh_1-1_Cue.Whoosh_1-1_Cue" (`self.K2_GetActorLocation`) (struct) 1.0 1.0 0.0 null null null null)
      (set `self.bCanThrowKnife` false)
      (`KismetSystemLibrary.Delay` 0.5)
      (set `self.bCanThrowKnife` true)
      (`SceneComponent.SetVisibility` (`self.Mesh`) true false))))

(event `ExcuteKnifeSpawn`
  (bind _returnvalue (`self.K2_GetActorRotation`))
  (`|SpawnActorFromClass` "/Game/Main/Weapon/BP_Throw_Knife.BP_Throw_Knife_C" (`KismetMathLibrary.MakeTransform` (+ (`SceneComponent.GetSocketLocation` (`self.HandDagger_Visual`) "Throw_Knife") (* (`KismetMathLibrary.GetForwardVector` _returnvalue) 200.0)) _returnvalue) "AlwaysSpawn" "MultiplyWithRoot" null null))

(event `Key|E`
  (params (Key :type "Key Structure"))
  (:`Pressed`
    (for _array_element (`self.GetOverlappingActors` null)
      (if (`KismetSystemLibrary.DoesImplementInterface` _array_element "/Game/Main/BPI_Interact.BPI_Interact_C")
        (message `/Game/Main/BPI_Interact.Interactor` _array_element self)))))

(event `AcquireThrowingKnifeSkill`
  (`self.OnDagger`)
  (`self.Change_Button_Z_Color`))

(event `AcquireUsingSwordSkill`
  (`self.OnSword`)
  (`self.Change_Button_X_Color`))

(event `Key|R`
  (params (Key :type "Key Structure"))
  (:`Pressed`
    (if (and (`self.bCanUseSword`) (not (`self.bIsAttacking`)))
      (`self.PlayAnimMontage` "/Game/Main/Weapon/AM_Sword.AM_Sword")
      (`GameplayStatics.PlaySoundAtLocation` "/Game/ShortSound/cue/Whoosh_4-1_Cue.Whoosh_4-1_Cue" (`self.K2_GetActorLocation`) (struct) 1.0 1.0 0.0 null null null null))))

(event `Key|Z`
  (params (Key :type "Key Structure"))
  (:`Pressed`
    (`self.OnDagger`)))

(event `Key|X`
  (params (Key :type "Key Structure"))
  (:`Pressed`
    (`self.OnSword`)))

(event `ActivateSwordCollision`
  (`KismetSystemLibrary.Delay` 0.5)
  (`ActorComponent.Activate` (`self.Sword_Collision`) false :!label _label)
  (`/Engine/EditorBlueprintResources/StandardMacros.DoOnce` false
    (:`Completed`
      (goto _label))))

(event `Key|C`
  (params (Key :type "Key Structure"))
  (:`Pressed`
    (`self.OffWeapon`)))

(event `DisableSwordCollision`
  (`ActorComponent.Deactivate` (`self.Sword_Collision`))
  (set `self.bIsAttacking` false))

(event `self.Sword_Collision.OnComponentBeginOverlap`
  (params (OverlappedComponent :type "PrimitiveComponent Object Reference") (OtherActor :type "Actor Object Reference") (OtherComp :type "PrimitiveComponent Object Reference") (OtherBodyIndex :type Integer) (bFromSweep :type Boolean) (SweepResult :type "HitResult Structure (by ref)"))
  (cast `/Game/Main/Assasin_BP/BP_Assasin` OtherActor
    (:`CastFailed`
      (`GameplayStatics.ApplyDamage` OtherActor 0.1 null self))))

(event `self.ReceiveAnyDamage`
  (params (Damage :type "Float (single-precision)") (DamageType :type "DamageType Object Reference") (InstigatedBy :type "Controller Object Reference") (DamageCauser :type "Actor Object Reference"))
  (bind _returnvalue (`KismetMathLibrary.Normal` (- (`self.K2_GetActorLocation` DamageCauser) (`self.K2_GetActorLocation`)) 20.0))
  (bind _output_get (set `self.HP` (- (`self.HP`) Damage)))
  (if (<= _output_get 0.0)
    (`self.PlayAnimMontage` "/Game/Main/Monster/MutantAnimation/AM_MutatntDIE.AM_MutatntDIE")
    (`KismetSystemLibrary.Delay` 2.0)
    (`self.K2_DestroyActor`)
    (else
      (`self.PlayAnimMontage` "/Game/Main/Assasin_BP/AM_AssasinDamage.AM_AssasinDamage")
      (`self.K2_SetActorLocation` _returnvalue)
      (`GameplayStatics.PlaySoundAtLocation` "/Game/ShortSound/cue/Shield_Metal_Impact_1-3_Cue.Shield_Metal_Impact_1-3_Cue" _returnvalue (struct) 1.0 1.0 0.0 null null null null))))

(fn `Change_Button_X_Color`
  (if (`self.bCanUseSword`)
    (set `ProgressBar.WidgetStyle` (`self.Style`) (`/Game/Main/Assasin_BP/UI_Assasin.BUTTON_X` (`self.UI`)))))

(fn `Change_Button_Z_Color`
  (if (`self.bCanThrowKnife`)
    (set `ProgressBar.WidgetStyle` (`self.Style`) (`/Game/Main/Assasin_BP/UI_Assasin.BUTTON_Z` (`self.UI`)))))

(fn `OffWeapon`
  (set `self.bCanThrowKnife` false)
  (`SceneComponent.SetVisibility` (`self.HandDagger_Visual`) false false)
  (set `self.bCanUseSword` false)
  (`SceneComponent.SetVisibility` (`self.Sword`) false false)
  (`PrimitiveComponent.SetCollisionEnabled` (`self.Sword_Collision`) "NoCollision")
  (set `CharacterMovementComponent.MaxWalkSpeed` 1000.0 (`self.CharacterMovement`)))

(fn `OnDagger`
  (set `self.bCanThrowKnife` true)
  (`SceneComponent.SetVisibility` (`self.HandDagger_Visual`) true false)
  (set `self.bCanUseSword` false)
  (`SceneComponent.SetVisibility` (`self.Sword`) false false)
  (`PrimitiveComponent.SetCollisionEnabled` (`self.Sword_Collision`) "NoCollision")
  (set `CharacterMovementComponent.MaxWalkSpeed` 800.0 (`self.CharacterMovement`))
  (`GameplayStatics.PlaySoundAtLocation` "/Engine/VREditor/Sounds/VR_ungrab_Cue.VR_ungrab_Cue" (`self.K2_GetActorLocation`) (struct) 1.0 1.0 0.0 null null null null))

(fn `OnSword`
  (set `self.bCanUseSword` true)
  (`SceneComponent.SetVisibility` (`self.Sword`) true false)
  (`PrimitiveComponent.SetCollisionEnabled` (`self.Sword_Collision`) "QueryOnly")
  (set `self.bCanThrowKnife` false)
  (`SceneComponent.SetVisibility` (`self.HandDagger_Visual`) false false)
  (set `CharacterMovementComponent.MaxWalkSpeed` 600.0 (`self.CharacterMovement`))
  (`GameplayStatics.PlaySoundAtLocation` "/Engine/VREditor/Sounds/VR_teleport_Cue.VR_teleport_Cue" (`self.K2_GetActorLocation`) (struct) 1.0 1.0 0.0 null null null null))

(fn `Set Aim Mode`
  (set `HUD.bShowHUD` true (`self.Target HUD`))
  (set `self.bIsAiming?` true)
  (set `SpringArmComponent.TargetArmLength` 110.0 (`self.SpringArm`))
  (`SceneComponent.K2_SetRelativeLocation` (`self.Camera`) (0.0 80.0 15.0) false false)
  (set `self.bUseControllerRotationYaw` true)
  (set `CharacterMovementComponent.bOrientRotationToMovement` false (`self.CharacterMovement`)))

(fn `Set Nav Mode`
  (set `HUD.bShowHUD` false (`self.Target HUD`))
  (set `self.bIsAiming?` false)
  (set `SpringArmComponent.TargetArmLength` 400.0 (`self.SpringArm`))
  (`SceneComponent.K2_SetRelativeLocation` (`self.Camera`) (0.0 0.0 0.0) false false)
  (set `self.bUseControllerRotationYaw` false)
  (set `CharacterMovementComponent.bOrientRotationToMovement` true (`self.CharacterMovement`)))

(fn `UserConstructionScript`)